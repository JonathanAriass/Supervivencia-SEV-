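; Orc enemy character that chases the player, attacks in melee and dies when its health runs out.
; A self-repeating AI MoveTo follows the player, while Tick raises walk speed when the player is far away.
; A looping timer checks range and plays the attack montage behind a DoOnce, hitting the player on completion.
; Impactado reduces health, then at zero disables mesh collision, plays the death montage and destroys the actor.
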(event `self.ReceiveBeginPlay`
  ;[1 1 1] Timer para los ataques del enemigo en este caso 0.3
  (bind _returnvalue (`GameplayStatics.GetActorOfClass` "/Game/Player/Jugador.Jugador_C"))
  (set `self.Jugador` _returnvalue)
  (`KismetSystemLibrary.Delay` 1.0)
  (`self.FollowPlayer`)
  (`KismetSystemLibrary.K2_SetTimerDelegate` (delegate `Attack`) 0.3 true))

(event `Attack`
  ;[1 1 1] Funcion para atacar al jugador dependiendo de la posicion y se reproduce el montage de ataque
  (bind _jugador (`self.Jugador`)
    (:`then`
      (if (<= (`self.GetDistanceTo` _jugador) 200.0)
        (`/Engine/EditorBlueprintResources/StandardMacros.DoOnce` false :!label _label
          (:`Completed`
            (`|PlayMontage` (`self.Mesh`) "/Game/Enemy/EnemyAmpliacion/OrcAttacking_Montage.OrcAttacking_Montage"
              (:`OnCompleted`
                (`|ExecutionSequence`
                  (:`then_0`
                    (`/Game/Player/Jugador.Impactado` (`self.Jugador`)))
                  (:`then_1`
                    (goto _label :!via `Reset`)))))))))
    (:`else`)))

(event `FollowPlayer`
  ;[1 1 1] Funcion para seguir al jugador (acordarse de usar la mesh para la zona de deteccion)
  (bind _jugador (`self.Jugador`)
    (:`then`
      (`|AIMoveTo` self (0.0 0.0 0.0) _jugador 100.0
        (:`OnSuccess`
          (`self.FollowPlayer`))))
    (:`else`)))

(event `Impactado`
  (bind _mesh (`self.Mesh`))
  ;[1 1 1] Animacion de morir
  (`self.Reducir Vida` 10)
  (if (<= (`self.Vida`) 0)
    (`PrimitiveComponent.SetCollisionEnabled` _mesh "NoCollision")
    (`|PlayMontage` _mesh "/Game/Enemy/EnemyAmpliacion/OrcDying_Montage.OrcDying_Montage"
      (:`then`
        (`KismetSystemLibrary.Delay` 2.65)
        (`self.K2_DestroyActor`)))))

(event `SetWalkSpeed`
  (bind _charactermovement (`self.CharacterMovement`))
  ;[1 1 1] Funcion para cambiar la velocidad del enemigo dependiendo de la posicion del jugador
  (bind _jugador (`self.Jugador`)
    (:`then`
      (if (> (`self.GetDistanceTo` _jugador) 750.0)
        (set `CharacterMovementComponent.MaxWalkSpeed` 500.0 _charactermovement)
        (else
          (set `CharacterMovementComponent.MaxWalkSpeed` 200.0 _charactermovement))))
    (:`else`)))

(event `self.ReceiveTick`
  (params (DeltaSeconds :type "Float (single-precision)"))
  ;[1 1 1] Funcion para cambiar la velocidad del enemigo dependiendo de la posicion del jugador
  (`self.SetWalkSpeed`))

(fn `UserConstructionScript`
  (`parent.UserConstructionScript`))