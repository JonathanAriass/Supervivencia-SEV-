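; Enemy actor that chases the player (Jugador) and attacks it at close range.
; After a short delay on BeginPlay it runs AIMoveTo toward the player, re-issuing the move each time it succeeds.
; A looping one-second timer calls Impactado on the player when within range and prints a debug string.
; Its own Impactado event reduces health (Vida) and destroys the actor at zero.
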(event `self.ReceiveBeginPlay`
  (bind _returnvalue (`GameplayStatics.GetActorOfClass` "/Game/Jugador.Jugador_C"))
  (set `self.Jugador` _returnvalue)
  (`KismetSystemLibrary.Delay` 1.0)
  (`self.FollowPlayer`)
  (`KismetSystemLibrary.K2_SetTimerDelegate` (delegate `Attack`) 1.0 true))

(event `FollowPlayer`
  (bind _jugador (`self.Jugador`)
    (:`then`
      (`|AIMoveTo` self (0.0 0.0 0.0) _jugador 100.0
        (:`OnSuccess`
          (`self.FollowPlayer`))))
    (:`else`)))

(event `Attack`
  (bind _jugador (`self.Jugador`)
    (:`then`
      (if (<= (`self.GetDistanceTo` _jugador) 200.0)
        (`/Game/Jugador.Impactado` (`self.Jugador`))
        (`KismetSystemLibrary.PrintString` "Hello")))
    (:`else`)))

(event `Impactado`
  (`self.Reducir Vida` 10)
  (if (<= (`self.Vida`) 0)
    (`self.K2_DestroyActor`)))

(fn `UserConstructionScript`
  (`parent.UserConstructionScript`))